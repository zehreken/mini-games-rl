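; Learning Agents training environment that defines rewards, episode completion and resets for the GoldRush minigame player agent.
; Each step rewards collections, penalizes misses and applies a small constant penalty, then clears the player's collected and missed flags.
; An episode terminates once the player's miss count exceeds a fixed limit, and resetting delegates to the player's own Reset function.
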(fn GatherAgentReward
  (params (AgentId :type Integer))
  (bind _output_get (LocalVariables|SetRewardActor (Class|LearningAgentsManagerListener|GetAgent AgentId "/Game/MiniGames/GoldRush/BP_GoldRushPlayer.BP_GoldRushPlayer_C")))
  (bind _output_get_2 (LocalVariables|SetReward (+ (Class|LearningAgentsRewards|MakeRewardonCondition (Variables|/Game/MiniGames/GoldRush/BP_GoldRushPlayer.BP_GoldRushPlayer_C|GetHasMissed (LocalVariables|GetRewardActor)) -0.5 "ConditionReward" false 0) (Class|LearningAgentsRewards|MakeRewardonCondition (Variables|/Game/MiniGames/GoldRush/BP_GoldRushPlayer.BP_GoldRushPlayer_C|GetHasCollected (LocalVariables|GetRewardActor)) 1.0 "ConditionReward" false 0) -0.001)))
  (Variables|/Game/MiniGames/GoldRush/BP_GoldRushPlayer.BP_GoldRushPlayer_C|SetHasCollected _output_get false)
  (Variables|/Game/MiniGames/GoldRush/BP_GoldRushPlayer.BP_GoldRushPlayer_C|SetHasMissed _output_get false)
  (return _output_get_2))

(fn GatherAgentCompletion
  (params (AgentId :type Integer))
  (return (Class|LearningAgentsCompletions|MakeCompletiononCondition (> (Variables|/Game/MiniGames/GoldRush/BP_GoldRushPlayer.BP_GoldRushPlayer_C|GetMissedCount (Class|LearningAgentsManagerListener|GetAgent AgentId "/Game/MiniGames/GoldRush/BP_GoldRushPlayer.BP_GoldRushPlayer_C")) 20) "Termination" "ConditionCompletion" false 0)))

(fn ResetAgentEpisode
  (params (AgentId :type Integer))
  (Default|Reset (Class|LearningAgentsManagerListener|GetAgent AgentId "/Game/MiniGames/GoldRush/BP_GoldRushPlayer.BP_GoldRushPlayer_C")))