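; BP_GoldRushPlayerInteractor is a Learning Agents interactor that defines what the GoldRush minigame player agent observes and how it acts.
; It observes the Y and Z offsets from the player to the nearest valid obstacle in the player's Obstacles array, normalized and clamped.
; Its single float "Direction" action is passed straight to the player's Move function.
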(fn SpecifyAgentObservation
  (params (InObservationSchema :type Learning%20Agents%20Observation%20Schema%20Object%20Reference))
  (return (Class|LearningAgentsObservations|SpecifyStructObservation InObservationSchema (Utilities|Map|MakeMap "RelativeYToObstacle" (Class|LearningAgentsObservations|SpecifyFloatObservation InObservationSchema 1.0) "RelativeZToObstacle" (Class|LearningAgentsObservations|SpecifyFloatObservation InObservationSchema 1.0)))))

(fn GatherAgentObservation
  (params (InObservationObject :type Learning%20Agents%20Observation%20Object%20Object%20Reference) (AgentId :type Integer))
  (bind _output_get (LocalVariables|SetObservedActor (Class|LearningAgentsManagerListener|GetAgent AgentId "/Game/MiniGames/GoldRush/BP_GoldRushPlayer.BP_GoldRushPlayer_C")))
  (bind _closestobstaclelocation (CallFunction|GetClosestObstacle (Variables|/Game/MiniGames/GoldRush/BP_GoldRushPlayer.BP_GoldRushPlayer_C|GetObstacles _output_get) _output_get))
  (LocalVariables|SetClosestObstacleLocation _closestobstaclelocation)
  (return (Class|LearningAgentsObservations|MakeStructObservation InObservationObject (Utilities|Map|MakeMap "RelativeYToObstacle" (Class|LearningAgentsObservations|MakeFloatObservation InObservationObject (Math|Float|Clamp(Float) (/ (.Y (Math|Vector|BreakVector (- (LocalVariables|GetClosestObstacleLocation) (Transformation|GetActorLocation (LocalVariables|GetObservedActor))))) 8e+02) -1.0) "FloatObservation" false 0) "RelativeZToObstacle" (Class|LearningAgentsObservations|MakeFloatObservation InObservationObject (Math|Float|Clamp(Float) (/ (.Z (Math|Vector|BreakVector (- (LocalVariables|GetClosestObstacleLocation) (Transformation|GetActorLocation (LocalVariables|GetObservedActor))))) 6.5e+02)) "FloatObservation" false 0)))))

(fn SpecifyAgentAction
  (params (InActionSchema :type Learning%20Agents%20Action%20Schema%20Object%20Reference))
  (return (Class|LearningAgentsActions|SpecifyFloatAction InActionSchema 1.0 "Direction")))

(fn PerformAgentAction
  (params (InActionObject :type Learning%20Agents%20Action%20Object%20Object%20Reference) (InActionObjectElement :type Learning%20Agents%20Action%20Object%20Element%20Structure%20%28by%20ref%29) (AgentId :type Integer))
  (Utilities|IsValid InActionObject
    (:Is%20Valid
      (bind _output_get (LocalVariables|SetActActor (Class|LearningAgentsManagerListener|GetAgent AgentId "/Game/MiniGames/GoldRush/BP_GoldRushPlayer.BP_GoldRushPlayer_C")))
      (bind _outvalue (Class|LearningAgentsActions|GetFloatAction InActionObject InActionObjectElement "Direction" false 0))
      (Default|Move _output_get _outvalue))
    (:Is%20Not%20Valid
      (Development|PrintString 0 "not valid" true true "(R=1.000000,G=0.000000,B=0.620994,A=1.000000)"))))

(fn GetClosestObstacle
  (params (Obstacles :type Array%20of%20BP%20Gold%20Rush%20Obstacle%20Object%20References) (Player :type BP%20Gold%20Rush%20Player%20Object%20Reference))
  (for _array_element Obstacles
    (Utilities|IsValid _array_element
      (:Is%20Valid
        (if (< (Transformation|GetDistanceTo _array_element Player) (LocalVariables|GetClosestDistance))
          (LocalVariables|SetClosestDistance (Transformation|GetDistanceTo _array_element Player))
          (LocalVariables|SetClosestLocation (Transformation|GetActorLocation _array_element))))))
  (return (LocalVariables|GetClosestLocation)))