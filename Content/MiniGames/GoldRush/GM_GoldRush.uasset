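; Game mode for the GoldRush minigame that sets up the player pawn and keeps obstacles coming.
; When a new player starts, it spawns a BP_GoldRushPlayer at a fixed low point and has the first player controller possess it.
; A looping timer spawns a BP_GoldRushObstacle at a random horizontal position higher up every few seconds.
; Each obstacle joins a growing array, which is then copied to the player pawn.
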(event Custom|SpawnActor
  (bind _returnvalue (Game|SpawnActorfromClass "/Game/MiniGames/GoldRush/BP_GoldRushObstacle.BP_GoldRushObstacle_C" (Math|Transform|MakeTransform (Math|Vector|MakeVector 0.0 (Math|Random|RandomFloatinRange -7.5e+02 7.5e+02) 3e+02)) "Undefined" "MultiplyWithRoot" 0 0))
  (Utilities|Array|Add (Variables|Default|GetObstacles) _returnvalue)
  (bind _asbp_gold_rush_player (Utilities|Casting|CastToBP_GoldRushPlayer (Game|Player|GetPlayerPawn 0)))
  (Variables|/Game/MiniGames/GoldRush/BP_GoldRushPlayer.BP_GoldRushPlayer_C|SetObstacles _asbp_gold_rush_player (Variables|Default|GetObstacles)))

(event EventBeginPlay
  (Utilities|Time|SetTimerbyEvent (delegate Custom|SpawnActor) 3.0 true))

(event EventTick
  (params (DeltaSeconds :type Float%20%28single-precision%29)))

(event EventHandleStartingNewPlayer
  (params (NewPlayer :type Player%20Controller%20Object%20Reference))
  (bind _returnvalue (Game|SpawnActorfromClass "/Game/MiniGames/GoldRush/BP_GoldRushPlayer.BP_GoldRushPlayer_C" (Math|Transform|MakeTransform (Math|Vector|MakeVector 0.0 0.0 -3e+02)) "AlwaysSpawn" "MultiplyWithRoot" 0 0))
  (Pawn|Possess (Game|GetPlayerController 0) _returnvalue))

(fn ConstructionScript)