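; Falling obstacle for the Reverse Kaboom minigame that makes the player lose on contact.
; Tick moves it down its local Z axis at a constant speed, without sweeping.
; On any actor overlap, it calls Lose if the other actor is the player, then removes itself from the game mode's Obstacles collection and destroys itself.
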(event EventBeginPlay)

(event Collision|EventActorBeginOverlap
  (params (OtherActor :type Actor%20Object%20Reference))
  (bind _asbp_reverse_kaboom_player (Utilities|Casting|CastToBP_ReverseKaboomPlayer OtherActor)
    (:then
      (Default|Lose _asbp_reverse_kaboom_player))
    (:CastFailed
      _))
  (bind _asgm_reverse_kaboom (Utilities|Casting|CastToGM_ReverseKaboom (Game|GetGameMode)))
  (Utilities|Array|RemoveItem (Variables|/Game/MiniGames/ReverseKaboom/GM_ReverseKaboom.GM_ReverseKaboom_C|GetObstacles _asgm_reverse_kaboom) self)
  (Actor|DestroyActor))

(event EventTick
  (params (DeltaSeconds :type Float%20%28single-precision%29))
  (Transformation|AddActorLocalOffset (* DeltaSeconds (Math|Vector|MakeVector 0.0 0.0 -2e+02)) false false))

(fn ConstructionScript)