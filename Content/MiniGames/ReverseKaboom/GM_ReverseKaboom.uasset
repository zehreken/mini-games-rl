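; Game mode for the Reverse Kaboom minigame that spawns the player pawn and a steady stream of obstacles.
; When a new player starts, it spawns a BP_ReverseKaboomPlayer at a fixed low point and has player controller 0 possess it.
; A fast looping timer spawns obstacles at random horizontal positions above, records them in an Obstacles array and copies that array to the player pawn.
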(event Custom|SpawnActor
  (bind _returnvalue (Game|SpawnActorfromClass "/Game/MiniGames/ReverseKaboom/BP_ReverseKaboomObstacle.BP_ReverseKaboomObstacle_C" (Math|Transform|MakeTransform (Math|Vector|MakeVector 0.0 (Math|Random|RandomFloatinRange -1e+03 1e+03) 3e+02)) "Undefined" "MultiplyWithRoot" 0 0))
  (Utilities|Array|Add (Variables|Default|GetObstacles) _returnvalue)
  (bind _asbp_reverse_kaboom_player (Utilities|Casting|CastToBP_ReverseKaboomPlayer (Game|Player|GetPlayerPawn 0)))
  (Variables|/Game/MiniGames/ReverseKaboom/BP_ReverseKaboomPlayer.BP_ReverseKaboomPlayer_C|SetObstacles _asbp_reverse_kaboom_player (Variables|Default|GetObstacles)))

(event EventBeginPlay
  (Utilities|Time|SetTimerbyEvent (delegate Custom|SpawnActor) 0.3 true))

(event EventTick
  (params (DeltaSeconds :type Float%20%28single-precision%29)))

(event EventHandleStartingNewPlayer
  (params (NewPlayer :type Player%20Controller%20Object%20Reference))
  (bind _returnvalue (Game|SpawnActorfromClass "/Game/MiniGames/ReverseKaboom/BP_ReverseKaboomPlayer.BP_ReverseKaboomPlayer_C" (Math|Transform|MakeTransform (Math|Vector|MakeVector 0.0 0.0 -3e+02)) "AlwaysSpawn" "MultiplyWithRoot" 0 0))
  (Pawn|Possess (Game|GetPlayerController 0) _returnvalue))

(fn ConstructionScript)