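; Learning Agents training environment that scores and resets BP_ReverseKaboomPlayer agents for reinforcement learning in the Reverse Kaboom minigame.
; Reward combines a bonus for passing, a larger penalty for being hit and a tiny constant per step.
; Gathering the reward clears the player's pass and hit flags, so each event counts once.
; An episode terminates once the hit count exceeds a fixed limit, and episode reset calls the player's Reset.
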(fn GatherAgentReward
  (params (AgentId :type Integer))
  (bind _output_get (LocalVariables|SetRewardActor (Class|LearningAgentsManagerListener|GetAgent AgentId "/Game/MiniGames/ReverseKaboom/BP_ReverseKaboomPlayer.BP_ReverseKaboomPlayer_C")))
  (bind _output_get_2 (LocalVariables|SetReward (+ (Class|LearningAgentsRewards|MakeRewardonCondition (Variables|/Game/MiniGames/ReverseKaboom/BP_ReverseKaboomPlayer.BP_ReverseKaboomPlayer_C|GetHasPassed (LocalVariables|GetRewardActor)) 0.5 "ConditionReward" false 0) (Class|LearningAgentsRewards|MakeRewardonCondition (Variables|/Game/MiniGames/ReverseKaboom/BP_ReverseKaboomPlayer.BP_ReverseKaboomPlayer_C|GetWasHit (LocalVariables|GetRewardActor)) -1.0 "ConditionReward" false 0) 0.001)))
  (Variables|/Game/MiniGames/ReverseKaboom/BP_ReverseKaboomPlayer.BP_ReverseKaboomPlayer_C|SetWasHit _output_get false)
  (Variables|/Game/MiniGames/ReverseKaboom/BP_ReverseKaboomPlayer.BP_ReverseKaboomPlayer_C|SetHasPassed _output_get false)
  (return _output_get_2))

(fn GatherAgentCompletion
  (params (AgentId :type Integer))
  (return (Class|LearningAgentsCompletions|MakeCompletiononCondition (> (Variables|/Game/MiniGames/ReverseKaboom/BP_ReverseKaboomPlayer.BP_ReverseKaboomPlayer_C|GetHitCount (Class|LearningAgentsManagerListener|GetAgent AgentId "/Game/MiniGames/ReverseKaboom/BP_ReverseKaboomPlayer.BP_ReverseKaboomPlayer_C")) 20) "Termination" "ConditionCompletion" false 0)))

(fn ResetAgentEpisode
  (params (AgentId :type Integer))
  (Default|Reset (Class|LearningAgentsManagerListener|GetAgent AgentId "/Game/MiniGames/ReverseKaboom/BP_ReverseKaboomPlayer.BP_ReverseKaboomPlayer_C")))