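; Learning Agents interactor for the Reverse Kaboom minigame, defining what a BP_ReverseKaboomPlayer agent observes and how it acts.
; It observes four floats: signed Y offsets to the left and right borders, plus Y and Z offsets to the player's current obstacle.
; A binary either action drives the player, with A calling MoveLeft and B calling MoveRight.
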(fn SpecifyAgentObservation
  (params (InObservationSchema :type Learning%20Agents%20Observation%20Schema%20Object%20Reference))
  (return (Class|LearningAgentsObservations|SpecifyStructObservation InObservationSchema (Utilities|Map|MakeMap "DistanceToLeftBorder" (Class|LearningAgentsObservations|SpecifyFloatObservation InObservationSchema 1.0) "DistanceToRightBorder" (Class|LearningAgentsObservations|SpecifyFloatObservation InObservationSchema 1.0) "RelativeYToObstacle" (Class|LearningAgentsObservations|SpecifyFloatObservation InObservationSchema 1.0) "RelativeZToObstacle" (Class|LearningAgentsObservations|SpecifyFloatObservation InObservationSchema 1.0)))))

(fn GatherAgentObservation
  (params (InObservationObject :type Learning%20Agents%20Observation%20Object%20Object%20Reference) (AgentId :type Integer))
  (LocalVariables|SetObsActor (Class|LearningAgentsManagerListener|GetAgent AgentId "/Game/MiniGames/ReverseKaboom/BP_ReverseKaboomPlayer.BP_ReverseKaboomPlayer_C"))
  (return (Class|LearningAgentsObservations|MakeStructObservation InObservationObject (Utilities|Map|MakeMap "DistanceToLeftBorder" (Class|LearningAgentsObservations|MakeFloatObservation InObservationObject (.Y (Math|Vector|BreakVector (- (LocalVariables|GetLeftBorder) (Transformation|GetActorLocation (LocalVariables|GetObsActor))))) "FloatObservation" false 0) "DistanceToRightBorder" (Class|LearningAgentsObservations|MakeFloatObservation InObservationObject (.Y (Math|Vector|BreakVector (- (LocalVariables|GetRigthBorder) (Transformation|GetActorLocation (LocalVariables|GetObsActor))))) "FloatObservation" false 0) "RelativeYToObstacle" (Class|LearningAgentsObservations|MakeFloatObservation InObservationObject (.Y (Math|Vector|BreakVector (- (Transformation|GetActorLocation (Variables|/Game/MiniGames/ReverseKaboom/BP_ReverseKaboomPlayer.BP_ReverseKaboomPlayer_C|GetCurrentObstacle (LocalVariables|GetObsActor))) (Transformation|GetActorLocation (LocalVariables|GetObsActor))))) "FloatObservation" false 0) "RelativeZToObstacle" (Class|LearningAgentsObservations|MakeFloatObservation InObservationObject (.Z (Math|Vector|BreakVector (- (Transformation|GetActorLocation (Variables|/Game/MiniGames/ReverseKaboom/BP_ReverseKaboomPlayer.BP_ReverseKaboomPlayer_C|GetCurrentObstacle (LocalVariables|GetObsActor))) (Transformation|GetActorLocation (LocalVariables|GetObsActor))))) "FloatObservation" false 0)))))

(fn SpecifyAgentAction
  (params (InActionSchema :type Learning%20Agents%20Action%20Schema%20Object%20Reference))
  (return (Class|LearningAgentsActions|SpecifyEitherAction InActionSchema)))

(fn PerformAgentAction
  (params (InActionObject :type Learning%20Agents%20Action%20Object%20Object%20Reference) (InActionObjectElement :type Learning%20Agents%20Action%20Object%20Element%20Structure%20%28by%20ref%29) (AgentId :type Integer))
  (LocalVariables|SetActActor (Class|LearningAgentsManagerListener|GetAgent AgentId "/Game/MiniGames/ReverseKaboom/BP_ReverseKaboomPlayer.BP_ReverseKaboomPlayer_C"))
  (Class|LearningAgentsActions|GetEitherAction InActionObject InActionObjectElement
    (:A
      (Default|MoveLeft (LocalVariables|GetActActor)))
    (:B
      (Default|MoveRight (LocalVariables|GetActActor)))))