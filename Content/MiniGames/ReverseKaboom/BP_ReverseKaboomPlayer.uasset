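; Player actor for the Reverse Kaboom minigame, sliding along a clamped Y range and tracking whether it gets hit.
; Move shifts it by a scaled direction input, any overlap sets WasHit, and Lose sets HasPassed and increments LostCount.
; Reset restores the start position and clears those states and the Obstacles list.
; Code to register it with a Learning Agents manager exists but is disconnected.
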(event EventBeginPlay)

(event Collision|EventActorBeginOverlap
  (params (OtherActor :type Actor%20Object%20Reference))
  (bind _output_get (Variables|Default|SetWasHit true)))

(event EventTick
  (params (DeltaSeconds :type Float%20%28single-precision%29)))

(fn ConstructionScript)

(fn Reset
  (Transformation|SetActorLocation "0.000000,0.000000,-300.000000" false false)
  (Variables|Default|SetWasHit false)
  (Variables|Default|SetHasPassed false)
  (Utilities|Array|Clear (Variables|Default|GetObstacles))
  (Variables|Default|SetLostCount 0))

(fn Move
  (params (Direction :type Float%20%28double-precision%29))
  (bind _returnvalue (Transformation|GetActorLocation))
  (bind (_x _y _z) (Math|Vector|BreakVector _returnvalue))
  (Transformation|SetActorLocation (Math|Vector|MakeVector _x (Math|Float|Clamp(Float) (+ _y (* Direction 1e+01)) -7.5e+02 7.5e+02) _z) false false))

(fn Lose
  (Variables|Default|SetHasPassed true)
  (Math|Integer|IncrementInt (Variables|Default|GetLostCount)))