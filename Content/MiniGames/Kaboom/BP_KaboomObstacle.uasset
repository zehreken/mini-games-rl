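; Falling obstacle actor for the Kaboom minigame that makes the player lose when it overlaps an actor.
; Tick moves it down its local Z axis at a constant, frame-rate-independent speed, without sweeping.
; Any overlap, with no check on the other actor, calls Lose on the found BP_KaboomPlayer, removes the obstacle from GM_Kaboom's Obstacles list and destroys it.
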(event EventBeginPlay)

(event Collision|EventActorBeginOverlap
  (params (OtherActor :type Actor%20Object%20Reference))
  (bind _returnvalue (Actor|GetActorOfClass "/Game/MiniGames/Kaboom/BP_KaboomPlayer.BP_KaboomPlayer_C"))
  (Default|Lose _returnvalue)
  (bind _asgm_kaboom (Utilities|Casting|CastToGM_Kaboom (Game|GetGameMode)))
  (Utilities|Array|RemoveItem (Variables|/Game/MiniGames/Kaboom/GM_Kaboom.GM_Kaboom_C|GetObstacles _asgm_kaboom) self)
  (Actor|DestroyActor))

(event EventTick
  (params (DeltaSeconds :type Float%20%28single-precision%29))
  (Transformation|AddActorLocalOffset (* DeltaSeconds (Math|Vector|MakeVector 0.0 0.0 -2e+02)) false false))

(fn ConstructionScript)